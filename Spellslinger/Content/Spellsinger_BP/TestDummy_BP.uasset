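; TestDummy_BP is a target dummy that takes damage and displays its current health as text.
; Both the Attacked event and player overlap with its Box, which deals fixed damage, feed ITookDamage.
; That function passes health and damage through TakeDamageAC, stores the result and updates HealthDisplay.
; When health is already depleted, the next hit restores it to BaseHealth instead of applying damage.
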(event `self.ReceiveBeginPlay`
  (`TextRenderComponent.K2_SetText` (`self.Health Display`) (`KismetTextLibrary.Conv_DoubleToText` (`self.BaseHealth`) "HalfToEven")))

(event `Attacked`
  (params (Damage :type "Float (double-precision)"))
  (`self.I Took Damage` Damage))

(event `self.Box.OnComponentBeginOverlap`
  (params (OverlappedComponent :type "PrimitiveComponent Object Reference") (OtherActor :type "Actor Object Reference") (OtherComp :type "PrimitiveComponent Object Reference") (OtherBodyIndex :type Integer) (bFromSweep :type Boolean) (SweepResult :type "HitResult Structure (by ref)"))
  (cast `/Game/FirstPerson/Blueprints/BP_FirstPersonCharacter` OtherActor)
  (`self.I Took Damage` 15.0))

(fn `I Took Damage`
  (params (Damage :type "Float (double-precision)"))
  (if (<= (`self.Health`) 0.0)
    (bind _output_get (set `self.Health` (`self.BaseHealth`)))
    (`TextRenderComponent.K2_SetText` (`self.Health Display`) (`KismetTextLibrary.Conv_DoubleToText` _output_get "HalfToEven"))
    (else
      (bind _new_health (`/Game/Spellsinger_BP/TakeDamage_AC.Damaged` (`self.TakeDamage_AC`) (`self.Health`) Damage))
      (bind _output_get_2 (set `self.Health` _new_health))
      (`TextRenderComponent.K2_SetText` (`self.Health Display`) (`KismetTextLibrary.Conv_DoubleToText` _output_get_2 "HalfToEven")))))

(fn `UserConstructionScript`)